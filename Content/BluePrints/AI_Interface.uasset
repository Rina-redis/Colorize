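; AI_Interface is a roaming AI pawn that spreads its mesh material to others on contact.
; It chains AIMoveTo calls to random reachable points, starting the next only when a move succeeds.
; When its capsule hits an AI_ToColor actor and CanColor is set, it casts that actor to AI_Interface, enables its CanColor and copies its own material onto it, so coloring can propagate.
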(event OnComponentHit(CapsuleComponent)
  (params (HitComponent :type Primitive%20Component%20Object%20Reference) (OtherActor :type Actor%20Object%20Reference) (OtherComp :type Primitive%20Component%20Object%20Reference) (NormalImpulse :type Vector :default "0, 0, 0") (Hit :type Hit%20Result%20Structure%20%28by%20ref%29))
  (Variables|Default|SetTestActor OtherActor)
  (if (== (Utilities|GetClass (Variables|Default|GetTestActor)) "/Game/BluePrints/AI_ToColor.AI_ToColor_C")
    (CallFunction|Colorize OtherActor)))

(event Custom|RandomRoam
  (AI|AIMoveTo self (.RandomLocation (AI|Navigation|GetRandomReachablePointinRadius (Transformation|GetActorLocation) 2.5e+03 0 0)) 0 5.0 false
    (:OnSuccess
      (CallFunction|RandomRoam))))

(event Custom|CustomMaterial
  (params (Material :type Material%20Interface%20Object%20Reference))
  (Rendering|Material|SetMaterial (Variables|Default|GetStaticMesh) 0 Material))

(event Custom|Colorize
  (params (NewParam :type Actor%20Object%20Reference))
  (if (Variables|Default|GetCanColor)
    (bind _output_get (Variables|Default|SetOther%20Actor NewParam))
    (bind _asai_interface (Utilities|Casting|CastToAI_Interface _output_get))
    (Variables|AI_Interface_C|SetCanColor _asai_interface true)
    (CallFunction|CustomMaterial _asai_interface (Rendering|Material|GetMaterial (Variables|Default|GetStaticMesh) 0))))

(event EventBeginPlay
  (CallFunction|RandomRoam))

(fn ConstructionScript)