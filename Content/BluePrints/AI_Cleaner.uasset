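; AI_Cleaner is a roaming AI that can strip color from AI_ToColor actors it bumps into.
; Each capsule hit calls RandomRoam, then calls Colorize on the hit actor if its own CanColor is set.
; Otherwise, it checks for an AI_ToColor class, casts to AI_Interface, applies the M_Basic_Wall material and clears that actor's CanColor.
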(event OnComponentHit(CapsuleComponent)
  (params (HitComponent :type Primitive%20Component%20Object%20Reference) (OtherActor :type Actor%20Object%20Reference) (OtherComp :type Primitive%20Component%20Object%20Reference) (NormalImpulse :type Vector :default "0, 0, 0") (Hit :type Hit%20Result%20Structure%20%28by%20ref%29))
  (CallFunction|RandomRoam)
  (if (Variables|Default|GetCanColor)
    (CallFunction|Colorize OtherActor)
    (else
      (Variables|Default|SetOther%20Actor_0_0 OtherActor)
      (if (Utilities|ClassIsChildOf (Utilities|GetClass (Variables|Default|GetOther%20Actor_0_0)) "/Game/BluePrints/AI_ToColor.AI_ToColor_C")
        (bind _asai_interface (Utilities|Casting|CastToAI_Interface (Variables|Default|GetOther%20Actor_0_0)))
        (Default|CustomMaterial _asai_interface "/Game/StarterContent/Materials/M_Basic_Wall.M_Basic_Wall")
        (Variables|/Game/BluePrints/AI_Interface.AI_Interface_C|SetCanColor _asai_interface false)))))

(event EventBeginPlay
  (|CallParentFunction) ; This node is disabled and will not be called.\nDrag off pins to build functionality.
)

(event Collision|EventActorBeginOverlap
  (params (OtherActor :type Actor%20Object%20Reference)))

(event EventTick
  (params (DeltaSeconds :type Float%20%28single-precision%29)))

(fn ConstructionScript
  (|CallParentFunction))